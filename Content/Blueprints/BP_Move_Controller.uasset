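; Movement controller component for BP_Crocodile that drives a crawl gait and procedural body sway through the owner's Control Rig.
; It receives four leg controllers, binds their step events, and starts crawling with diagonal pairs initialized in offset phases.
; Each tick, a looping float curve drives body yaw, roll and pitch controls.
; Step-driven neck rotation is implemented but disconnected, and the PerformingStep handler is empty.
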(event Custom|InitializeLegControllers
  (params (LeftLeg :type BP%20Leg%20Controller%20Object%20Reference) (RightLeg :type BP%20Leg%20Controller%20Object%20Reference) (LeftLimb :type BP%20Leg%20Controller%20Object%20Reference) (RightLimb :type BP%20Leg%20Controller%20Object%20Reference))
  (Variables|Default|SetLeftLeg LeftLeg)
  (Variables|Default|SetRightLeg RightLeg)
  (Variables|Default|SetLeftLimb LeftLimb)
  (Variables|Default|SetRightLimb RightLimb)
  (EventDispatchers|BindEventtoOnPerformingStep (Variables|Default|GetLeftLeg) (EventDispatchers|CreateEvent :!event Custom|PerformingStep))
  (EventDispatchers|BindEventtoOnPerformingStep (Variables|Default|GetRightLeg) (EventDispatchers|CreateEvent :!event Custom|PerformingStep))
  (EventDispatchers|BindEventtoOnPerformingStep (Variables|Default|GetLeftLimb) (EventDispatchers|CreateEvent :!event Custom|PerformingStep))
  (EventDispatchers|BindEventtoOnPerformingStep (Variables|Default|GetRightLimb) (EventDispatchers|CreateEvent :!event Custom|PerformingStep))
  (CallFunction|InitializeAdditionalControllers))

(event Custom|StartCrawlGait
  (params (speed :type Float%20%28double-precision%29))
  ;[1 1 1] Initializing Movement with Crawl pattern and current speed
  (Default|InitializeLegwithValuesandState (Variables|Default|GetLeftLimb) 0.0 "NewEnumerator1" 0.35 0.0)
  (Default|InitializeLegwithValuesandState (Variables|Default|GetRightLeg) 0.0 "NewEnumerator1" 0.35 0.0)
  (Default|InitializeLegwithValuesandState (Variables|Default|GetLeftLeg) 0.15 "NewEnumerator0" 0.35 0.0)
  (Default|InitializeLegwithValuesandState (Variables|Default|GetRightLimb) 0.15 "NewEnumerator0" 0.35 0.0))

(event Custom|PerformingStep
  (params (LegType :type E_LegType%20Enum :default "NewEnumerator0") (PercentageReplanted :type Float%20%28double-precision%29)))

(event Custom|InitializeAdditionalControllers
  (Variables|Default|SetTopSpineJoint (Class|ControlRigComponent|GetControlRotator (Variables|Default|GetControlRig) "NeckRotationCtrl" "LocalSpace")))

(event EventBeginPlay
  (Utilities|FlowControl|DelayUntilNextTick)
  (bind _asbp_crocodile (Utilities|Casting|CastToBP_Crocodile (Components|GetOwner)))
  (Variables|Default|SetControlRig (Variables|/Game/Blueprints/BP_Crocodile.BP_Crocodile_C|GetControlRig _asbp_crocodile)))

(event EventTick
  (params (DeltaSeconds :type Float%20%28single-precision%29))
  (CallFunction|PerformBodyRotation))

(fn PerformNeckRotation
  (bind _leftleg (Variables|Default|GetLeftLeg))
  (bind _rightleg (Variables|Default|GetRightLeg))
  (Class|ControlRigComponent|SetControlRotator (Variables|Default|GetControlRig) "NeckRotationCtrl" (Math|Rotator|MakeRotator 0.0 0.0 (* (- (- (/ (Variables|/Game/Blueprints/BP_LegController.BP_LegController_C|GetCurrentStepLengthSeconds _leftleg) (Variables|/Game/Blueprints/BP_LegController.BP_LegController_C|GetStepLengthSeconds _leftleg)) (/ (Variables|/Game/Blueprints/BP_LegController.BP_LegController_C|GetTimeSinceUnplanted _leftleg) (Variables|/Game/Blueprints/BP_LegController.BP_LegController_C|GetSwingStepTime _leftleg))) (- (/ (Variables|/Game/Blueprints/BP_LegController.BP_LegController_C|GetCurrentStepLengthSeconds _rightleg) (Variables|/Game/Blueprints/BP_LegController.BP_LegController_C|GetStepLengthSeconds _rightleg)) (/ (Variables|/Game/Blueprints/BP_LegController.BP_LegController_C|GetTimeSinceUnplanted _rightleg) (Variables|/Game/Blueprints/BP_LegController.BP_LegController_C|GetSwingStepTime _rightleg)))) (Variables|Parameters|GetNeckAngleRotationMax))) "LocalSpace"))

(fn PerformBodyRotation
  (bind _output_get (Variables|Default|SetTotalTime (+ (Variables|Default|GetTotalTime) (Utilities|Time|GetWorldDeltaSeconds))))
  (bind _output_get_2 (LocalVariables|SetCurveValue (Math|Curves|GetFloatValue (Variables|Parameters|GetNeckRotationCurve) (* (.Remainder (Math|Float|Division(WholeandRemainder) _output_get 1.0)) 2.0))))
  (Class|ControlRigComponent|SetControlRotator (Variables|Default|GetControlRig) "BodyRotationCtrl2" (Math|Rotator|MakeRotator 0.0 0.0 (* (LocalVariables|GetCurveValue) -15.0)) "LocalSpace")
  (Class|ControlRigComponent|SetControlRotator (Variables|Default|GetControlRig) "BodyHarmonics" (Math|Rotator|MakeRotator (+ (* (LocalVariables|GetCurveValue) -5.0) 9e+01) (* (LocalVariables|GetCurveValue) 1e+01) 0.0) "LocalSpace"))