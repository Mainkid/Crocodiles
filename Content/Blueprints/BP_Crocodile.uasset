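; Crocodile actor that crawls with a Control Rig body, a simulated-physics tail and a gait controller coordinating leg and limb controllers.
; Holding X or Z bends the BodyRotationCtrl yaw in opposite directions, and each Tick drives capsule velocity along the mesh's axis rotated by that bend.
; PoseRecovery eases the bend back each frame while counter-adjusting the mesh's local rotation, turning the body gradually.
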(event OnPreInitializeDelegate(ControlRig)
  (params (Component :type Control%20Rig%20Component%20Object%20Reference))
  (Class|ControlRigComponent|AddMappedCompleteSkeletalMesh Component (Variables|Default|GetSkeletalMesh)))

(event Custom|Move)

(event EventBeginPlay
  (Class|SkeletalMeshComponent|SetAllBodiesBelowSimulatePhysics (Variables|Default|GetSkeletalMesh) (Utilities|Name|MakeLiteralName "Crocodile_TailBase") true false)
  (Default|InitializeLegControllers (Variables|Default|GetBP_GAIT_Controller) (Variables|Default|GetBP_LeftLegController) (Variables|Default|GetBP_RightLegController) (Variables|Default|GetBP_LeftLimbController) (Variables|Default|GetBP_RightLimbController))
  (Default|StartCrawlGait (Variables|Default|GetBP_GAIT_Controller) 0.0))

(event EventTick
  (params (DeltaSeconds :type Float%20%28single-precision%29))
  (bind _controlrig (Variables|Default|GetControlRig))
  (bind _controlrig_2 (Variables|Default|GetControlRig))
  (bind _skeletalmesh (Variables|Default|GetSkeletalMesh))
  (bind _controlrig_3 (Variables|Default|GetControlRig))
  (bind _returnvalue (Class|ControlRigComponent|GetControlRotator _controlrig_2 "BodyRotationCtrl" "RigSpace"))
  (bind _returnvalue_2 (Math|Vector|GetUpVector _skeletalmesh))
  (bind _returnvalue_3 (* _returnvalue 0.75))
  (bind _returnvalue_4 (* _returnvalue_2 -1.0))
  (bind _returnvalue_5 (Math|Vector|RotateVector _returnvalue_4 _returnvalue_3))
  (Utilities|FlowControl|Sequence
    (:then_0
      (Physics|SetPhysicsLinearVelocity (Variables|Default|GetCapsule) (* _returnvalue_5 (Variables|Default|GetVelocity)) false "Crocodile_Tail_01_03SHJnt")
      (Variables|Default|SetMovementVector _returnvalue_5)
      (Development|PrintString (Utilities|String|ToString(Float) 0.0)))
    (:then_1
      (if (> (Class|PlayerController|GetInputKeyTimeDown (Game|GetPlayerController 0) "X") 0.0)
        (Class|ControlRigComponent|SetControlRotator _controlrig_3 "BodyRotationCtrl" (Math|Rotator|MakeRotator 0.0 0.0 (+ (.yaw (Class|ControlRigComponent|GetControlRotator _controlrig_3 "BodyRotationCtrl" "LocalSpace")) (* (Utilities|Time|GetWorldDeltaSeconds) 2e+01))) "LocalSpace")))
    (:then_2
      (if (> (Class|PlayerController|GetInputKeyTimeDown (Game|GetPlayerController 0) "Z") 0.0)
        (Class|ControlRigComponent|SetControlRotator _controlrig "BodyRotationCtrl" (Math|Rotator|MakeRotator 0.0 0.0 (+ (.yaw (Class|ControlRigComponent|GetControlRotator _controlrig "BodyRotationCtrl" "LocalSpace")) (* (Utilities|Time|GetWorldDeltaSeconds) -2e+01))) "LocalSpace")))
    (:then_3
      (CallFunction|PoseRecovery))))

(fn ConstructionScript)

(fn PoseRecovery
  (bind _controlrig (Variables|Default|GetControlRig))
  (Class|ControlRigComponent|SetControlRotator (Variables|Default|GetControlRig) "BodyRotationCtrl" (Math|Rotator|MakeRotator 0.0 0.0 (* (.yaw (Class|ControlRigComponent|GetControlRotator _controlrig "BodyRotationCtrl" "LocalSpace")) 0.99 1.0 1.0)) "LocalSpace")
  (Transformation|AddLocalRotation (Variables|Default|GetSkeletalMesh) (Math|Rotator|MakeRotator 0.0 (* (.yaw (Class|ControlRigComponent|GetControlRotator _controlrig "BodyRotationCtrl" "LocalSpace")) -0.01 1.0 1.0) 0.0) false false))